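; BP_MazeDoor is a color-coded locked door for the maze that opens when a player holding the matching key interacts with it.
; Interact casts the actor to BP_ThirdPersonCharacter and checks its Keys for the door's ColorName.
; On a match, a Timeline lerps the cube mesh's yaw or roll to swing it open; otherwise it prints a wrong-key message.
; The construction script applies the Color material to the mesh.
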(event EventInteract
  (params (InteractingActor :type Actor%20Object%20Reference))
  (bind _asbp_third_person_character (Utilities|Casting|CastToBP_ThirdPersonCharacter InteractingActor))
  (if (Utilities|Array|ContainsItem (Variables|/Game/ThirdPerson/Blueprints/BP_ThirdPersonCharacter.BP_ThirdPersonCharacter_C|GetKeys _asbp_third_person_character) (Variables|Default|GetColorName))
    (bind _newtrack_0 (Timeline|Timeline Play)
      (:Update
        (Transformation|SetRelativeRotation (Variables|Default|GetSM_Cube) (Math|Rotator|Lerp(Rotator) "0, 0, 0" "0.000000,-90.000000,0.000000" _newtrack_0) false false)))
    (else
      (Development|PrintString "Wrong Key"))))

(fn ConstructionScript
  (Rendering|Material|SetMaterial (Variables|Default|GetSM_Cube) 0 (Variables|Default|GetColor)))

(fn GaynessAnswer
  (return false))