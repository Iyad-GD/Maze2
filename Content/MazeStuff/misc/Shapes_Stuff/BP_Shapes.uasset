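; BP_Shapes is a shape actor that registers itself in the third-person game mode's AllShapes list on BeginPlay.
; Its Construction Script picks one of three shape types at random, then applies that data table row's mesh and name label, ending on the emissive material.
; ToggleSelection swaps between emissive and normal materials to show selection, and MoveShape offsets the actor along local X or Z.
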(event Custom|ToggleSelection
  (params (MakeSelected :type Boolean))
  (bind _staticmesh (Variables|Default|GetStaticMesh))
  (bind _st_shapes (Variables|Default|GetST_Shapes))
  (if MakeSelected
    (Rendering|Material|SetMaterial _staticmesh 0 (.emmesivematerial _st_shapes))
    (else
      (Rendering|Material|SetMaterial _staticmesh 0 (.normalmaterial _st_shapes)))))

(event Custom|MoveShape
  (params (Amount :type Float%20%28double-precision%29) (Horizontal? :type Boolean))
  (if Horizontal?
    (Transformation|AddActorLocalOffset (Math|Vector|MakeVector Amount 0.0 0.0) false false)
    (else
      (Transformation|AddActorLocalOffset (Math|Vector|MakeVector 0.0 0.0 Amount) false false))))

(event EventBeginPlay
  (bind _asbp_third_person_game_mode (Utilities|Casting|CastToBP_ThirdPersonGameMode (Game|GetGameMode)))
  (Utilities|Array|Add (Variables|/Game/ThirdPerson/Blueprints/BP_ThirdPersonGameMode.BP_ThirdPersonGameMode_C|GetAllShapes _asbp_third_person_game_mode) self))

(fn ConstructionScript
  (bind _staticmesh (Variables|Default|GetStaticMesh))
  (bind _output_get (Variables|Default|SetShapeType_0 (Utilities|Array|Get(acopy) (Variables|Default|GetShapeType) (Math|Random|RandomIntegerinRange 0 2))))
  (bind _returnvalue (Utilities|GetDataTableRow (Variables|Default|GetTable) (Utilities|String|StringToName (Utilities|String|EnumtoString _output_get)))
    (:then
      (bind _output_get_2 (Variables|Default|SetST_Shapes _returnvalue))
      (Components|StaticMesh|SetStaticMesh _staticmesh (.shapemesh _output_get_2))
      (Rendering|Material|SetMaterial _staticmesh 0 (.normalmaterial _output_get_2))
      (Rendering|Material|SetMaterial _staticmesh 0 (.emmesivematerial _output_get_2))
      (Rendering|Components|TextRender|SetText (Variables|Default|GetTextRender) (Utilities|Text|ToText(String) (.shapename _output_get_2))))))