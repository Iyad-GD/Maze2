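; Debug-style enemy spawn manager that spawns and damages test enemies from player key presses.
; F picks a random enemy type, looks up its difficulty in a map and its stats in DT_EnemyStats by enum name, printing both.
; It then spawns BP_EnemyBase at a random XY position with that data and stores it in an array.
; X damages every still-valid spawned enemy by a fixed amount.
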(event EventBeginPlay
  ;[0.15 0.15 0.15 0.5] Input Enable
  (Input|EnableInput (Game|GetPlayerController 0)))

(event Input|KeyboardEvents|F
  (params (Key :type Key%20Structure :default "None"))
  (:Pressed
    (bind _output_get (Variables|Default|SetSpawnEnemy (Utilities|Array|Get(acopy) (Variables|Default|GetEEnemyTypes) (Math|Random|RandomIntegerinRange 0 3))))
    (bind _output_get_2 (Variables|Default|SetSpawnedDifficulty (.Value (Utilities|Map|Find (Variables|Default|GetEnemyDificulty) (Variables|Default|GetSpawnEnemy)))))
    (Development|PrintString (Utilities|String|Append "Type: " (Utilities|String|EnumtoString _output_get) " Difficulty: " (Utilities|String|ToString(Integer) _output_get_2)))
    (bind _returnvalue (Utilities|GetDataTableRow "/Game/MazeStuff/misc/DT_EnemyStats.DT_EnemyStats" (Utilities|String|StringToName (Utilities|String|EnumtoString (Variables|Default|GetSpawnEnemy))))
      (:then
        (bind _output_get_3 (Variables|Default|SetEnemyStats _returnvalue))
        (Development|PrintString (Utilities|String|Append (Utilities|String|ToString(Float) (.health _output_get_3)) (Utilities|String|ToString(Float) (.damage _output_get_3)) (Utilities|String|ToString(Float) (.speed _output_get_3))))
        (bind _returnvalue_2 (Game|SpawnActorfromClass "/Game/MazeStuff/misc/BP_EnemyBase.BP_EnemyBase_C" (Math|Transform|MakeTransform (Math|Vector|MakeVector (Math|Random|RandomFloatinRange 0.0 1e+03) (Math|Random|RandomFloatinRange 0.0 1e+03) 92.0) "0, 0, 0" "1.000000,1.000000,1.000000") "Undefined" "MultiplyWithRoot" 0 (Variables|Default|GetSpawnEnemy) (Variables|Default|GetEnemyStats) (Variables|Default|GetSpawnedDifficulty) 0))
        (Utilities|Array|Add (Variables|Default|GetSpawnedEnemy) _returnvalue_2)))))

(event Input|KeyboardEvents|X
  (params (Key :type Key%20Structure :default "None"))
  (:Pressed
    (for _array_element (Variables|Default|GetSpawnedEnemy)
      (Utilities|IsValid _array_element
        (:Is%20Valid
          (Default|TakeDamage _array_element 5e+01))))))

(fn ConstructionScript)