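; BP_MazeCell is a configurable maze tile with four walls, a roof and a spotlight.
; The construction script sets light intensity and color, toggles roof and wall visibility from per-instance variables, and enables each wall's collision only when that wall is visible.
; ChangeRed and ChangeGreen events recolor the spotlight at runtime.
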(event Custom|ChangeRed
  (Rendering|Components|Light|SetLightColor (Variables|Default|GetSpotLight) "(R=0.875000,G=0.000000,B=0.044926,A=1.000000)" true))

(event Custom|ChangeGreen
  (Rendering|Components|Light|SetLightColor (Variables|Default|GetSpotLight) "(R=0.000000,G=1.000000,B=0.085974,A=1.000000)" true))

(fn ConstructionScript
  (bind _south_w (Variables|Default|GetSouth_W))
  (bind _east_w (Variables|Default|GetEast_W))
  (bind _west_w (Variables|Default|GetWest_W))
  (bind _spotlight (Variables|Default|GetSpotLight))
  (bind _north_w (Variables|Default|GetNorth_W))
  (Rendering|Components|Light|SetIntensity _spotlight (Variables|Adjustables|GetLight%20Intensity))
  (Rendering|Components|Light|SetLightColor _spotlight (Variables|Adjustables|GetLightColor) true)
  (Rendering|SetVisibility (Variables|Default|GetRoof) (Variables|Adjustables|GetCeiling) true)
  (Rendering|SetVisibility _north_w (Variables|Adjustables|GetNorthWall) true)
  (if (Rendering|IsVisible _north_w)
    (Collision|SetCollisionEnabled _north_w "QueryAndPhysics")
    (else
      (Collision|SetCollisionEnabled _north_w "NoCollision")))
  (Rendering|SetVisibility _south_w (Variables|Adjustables|GetSouthWall) true)
  (if (Rendering|IsVisible _south_w)
    (Collision|SetCollisionEnabled _south_w "QueryAndPhysics")
    (else
      (Collision|SetCollisionEnabled _south_w "NoCollision")))
  (Rendering|SetVisibility _east_w (Variables|Adjustables|GetEastWall) true)
  (if (Rendering|IsVisible _east_w)
    (Collision|SetCollisionEnabled _east_w "QueryAndPhysics")
    (else
      (Collision|SetCollisionEnabled _east_w "NoCollision")))
  (Rendering|SetVisibility _west_w (Variables|Adjustables|GetWestWall) true)
  (if (Rendering|IsVisible _west_w)
    (Collision|SetCollisionEnabled _west_w "QueryAndPhysics")
    (else
      (Collision|SetCollisionEnabled _west_w "NoCollision"))))