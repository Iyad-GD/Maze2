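; BP_EnemyBase is a base enemy actor that moves in a straight line and can be damaged until destroyed.
; BeginPlay copies health, damage and speed from EnemyStats and sets a text label showing enemy type and starting health.
; Tick offsets it along world X, scaled by speed and delta time.
; TakeDamage subtracts health, then destroys the actor at zero or below, otherwise returns the remaining health.
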(event EventBeginPlay
  (bind _enemystats (Variables|Default|GetEnemyStats))
  (bind _output_get (Variables|Default|SetCurrentHealth (.health _enemystats)))
  (Variables|Default|SetAttackDamage (.damage _enemystats))
  (Variables|Default|SetMoveSpeed (.speed _enemystats))
  (Rendering|Components|TextRender|SetText (Variables|Default|GetTextRender) (Utilities|Text|ToText(String) (Utilities|String|Append (Utilities|String|EnumtoString (Variables|Default|GetE_EnemyType)) "/" (Utilities|String|ToString(Float) _output_get)))))

(event EventTick
  (params (DeltaSeconds :type Float%20%28single-precision%29))
  (Transformation|AddActorWorldOffset (Math|Vector|MakeVector (* DeltaSeconds (Variables|Default|GetMoveSpeed) 5e+01) 0.0 0.0)))

(fn ConstructionScript)

(fn TakeDamage
  (params (Damage :type Float%20%28double-precision%29))
  (bind _output_get (Variables|Default|SetCurrentHealth (- (Variables|Default|GetCurrentHealth) Damage)))
  (if (<= _output_get 0.0)
    (Actor|DestroyActor)
    (else
      (return _output_get))))