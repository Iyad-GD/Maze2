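; BP_MazeDoor is a keyed maze door that swings open when it receives the correct key.
; WhichKey? stores the supplied key, and the test event compares it to DoorKey.
; A match plays a timeline that rotates the cube mesh 90 degrees, while a mismatch prints a wrong-key message.
; The construction script applies a configurable material to the mesh, and a separate answer function always returns false.
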(event EventGaynessTest
  (if (== (Variables|Default|GetKey) (Variables|Default|GetDoorKey))
    (bind _newtrack_0 (Timeline|Timeline Play)
      (:Update
        (Transformation|SetRelativeRotation (Variables|Default|GetSM_Cube) (Math|Rotator|Lerp(Rotator) "0, 0, 0" "0.000000,-90.000000,0.000000" _newtrack_0) false false)))
    (else
      (Development|PrintString "Wrong Key"))))

(fn ConstructionScript
  (Rendering|Material|SetMaterial (Variables|Default|GetSM_Cube) 0 (Variables|Default|GetMaterial)))

(fn GaynessAnswer
  (return false))

(fn WhichKey?
  (params (Value :type Integer))
  (bind _output_get (Variables|Default|SetKey Value))
  (return _output_get))